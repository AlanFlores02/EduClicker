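; Background actor for a find-the-Luigi game that tints its sprite while clicked and also manages scoring and rounds.
; On BeginPlay it creates the score HUD, which LuigiFound updates while counting down the remaining Luigis.
; When none remain, it resets every Item_BP and randomly turns items into Luigis at one-in-item-count odds each, forcing at least one per round.
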(event `self.RenderComponent.OnClicked`
  (params (TouchedComponent :type "PrimitiveComponent Object Reference") (ButtonPressed :type "Key Structure"))
  ;[0 0.2 0.8] Interactive
  (`PaperSpriteComponent.SetSpriteColor` (`self.RenderComponent`) (`self.Color Warp`)))

(event `self.RenderComponent.OnReleased`
  (params (TouchedComponent :type "PrimitiveComponent Object Reference") (ButtonReleased :type "Key Structure"))
  ;[0 0.2 0.8] Interactive
  (`PaperSpriteComponent.SetSpriteColor` (`self.RenderComponent`) (struct :`R` 1.0 :`G` 1.0 :`B` 1.0 :`A` 1.0)))

(event `self.ReceiveBeginPlay`
  (bind _returnvalue (`|CreateWidget` "/Game/HUD/HUD_Score.HUD_Score_C" (`GameplayStatics.GetPlayerController` 0)))
  (bind _output_get (set `self.HUD` _returnvalue))
  (`UserWidget.AddToViewport` _output_get 0))

(fn `Luigi Found`
  ;[0 0.2 0] Luigi Found
  (`/Game/HUD/HUD_Score.Score!` (`self.HUD`))
  (bind _result (`/Engine/EditorBlueprintResources/StandardMacros.DecrementInt` (`self.Luigis Left`))
    (:`  `
      (if (<= _result 0)
        ;[0.2 0.8 0.2] New Round
        (bind _outactors (`GameplayStatics.GetAllActorsOfClass` "/Game/Items/Item_BP.Item_BP_C"))
        (for _array_element _outactors
          (`/Game/Items/Item_BP.Reset` _array_element)
          (bind _returnvalue (`KismetMathLibrary.RandomInteger` (`KismetArrayLibrary.Array_Length` _outactors)))
          ;[1 1 1] Set Random Luigis
          (if (== 0 _returnvalue)
            (`/Game/Items/Item_BP.Return To Luigi` _array_element)
            (`/Engine/EditorBlueprintResources/StandardMacros.IncrementInt` (`self.Luigis Left`) :!label _label)))
        ;[0.25 0.25 0.25] Force at least one Luigi
        (if (== 0 (`self.Luigis Left`))
          (`/Game/Items/Item_BP.Return To Luigi` (`|GetArrayItem` _outactors _returnvalue))
          (goto _label))))))

(fn `UserConstructionScript`)