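; Player cursor actor that clicks on objects in what appears to be a find-Luigi game.
; Click runs a short visibility line trace along negative Y from its Niagara component and applies damage to whatever it hits.
; When the cursor itself takes damage, it reports LuigiFound with its IsPlayerOne flag to the Background_BP cached at BeginPlay, so damage serves as the messaging channel.
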(event `Click`
  (bind _returnvalue (`SceneComponent.K2_GetComponentLocation` (`self.Niagara`)))
  ;[1 1 1] Comment
  (bind (_outhit _returnvalue_2) (`KismetSystemLibrary.LineTraceSingle` _returnvalue (+ (0.0 -100.0 0.0) _returnvalue) "TraceTypeQuery1"))
  (if _returnvalue_2
    (`GameplayStatics.ApplyDamage` (`.HitActor` (`GameplayStatics.BreakHitResult` _outhit)) 1.0 null self)))

(event `self.ReceiveBeginPlay`
  (bind _returnvalue (`GameplayStatics.GetActorOfClass` "/Game/Background/Background_BP.Background_BP_C"))
  (set `self.Engine` _returnvalue))

(event `self.ReceiveAnyDamage`
  (params (Damage :type "Float (single-precision)") (DamageType :type "DamageType Object Reference") (InstigatedBy :type "Controller Object Reference") (DamageCauser :type "Actor Object Reference"))
  (`/Game/Background/Background_BP.Luigi Found` (`self.Engine`) (`self.Is Player One`)))

(fn `UserConstructionScript`)