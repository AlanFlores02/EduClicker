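; Player pawn or controller Blueprint that spawns and drives on-screen cursors for one or two local players.
; On BeginPlay it spawns Player 1's cursor and, when the GameInstance flags multiplayer, shows Player 2's HUD stats and spawns a re-skinned, recolored Wario cursor.
; Tick moves each cursor from its own axis input, with a Gate enabling Player 2's movement only in multiplayer.
; SpaceBar and J trigger each cursor's Click.
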(event `self.ReceiveBeginPlay`
  ;[0.5 0 1] Setup Player 1
  (bind _returnvalue (`|SpawnActorFromClass` "/Game/Player/Cursor_BP.Cursor_BP_C" (`KismetMathLibrary.MakeTransform` (0.0 10.0 0.0)) "AlwaysSpawn" "OverrideRootScale" null null))
  (set `self.Player 1` _returnvalue)
  ;[1 1 1] Use Player 2's UI
  (bind _asmy_game_instance (cast `/Game/Player/Settings/MyGameInstance` (`GameplayStatics.GetGameInstance`)))
  (if (`/Game/Player/Settings/MyGameInstance.Multiplayer?` _asmy_game_instance)
    (bind _returnvalue_2 (`GameplayStatics.GetActorOfClass` "/Game/Background/Background_BP.Background_BP_C"))
    (`Widget.SetRenderOpacity` (`/Game/HUD/HUD_Score.Player2_Stats` (`/Game/Background/Background_BP.HUD` _returnvalue_2)) 1.0)
    ;[1 0.8 0] Setup Player 2
    (bind _returnvalue_3 (`|SpawnActorFromClass` "/Game/Player/Cursor_BP.Cursor_BP_C" (`KismetMathLibrary.MakeTransform` (0.0 10.0 0.0)) "AlwaysSpawn" "OverrideRootScale" null null))
    (bind _output_get (set `self.Player 2` _returnvalue_3))
    (`PaperSpriteComponent.SetSprite` (`PaperSpriteActor.RenderComponent` _output_get) "/Game/Player/Sprites/Cursor_Wario_Sprite.Cursor_Wario_Sprite")
    (set `/Game/Player/Cursor_BP.Color Code` (struct :`R` 1.0 :`G` 0.875 :`B` 0.5 :`A` 1.0) _output_get)
    (set `/Game/Player/Cursor_BP.Is Player One` false _output_get)
    (goto _label :!via `Open`)))

(event `self.ReceiveTick`
  (params (DeltaSeconds :type "Float (single-precision)"))
  (bind _returnvalue (* DeltaSeconds (`self.Cursor Speed`)))
  ;[0 1 0] Cursor Movement
  (`self.K2_AddActorWorldOffset` (`self.Player 1`) (* (`KismetMathLibrary.MakeVector` (`self.GetInputAxisValue`) 0.0 (`self.GetInputAxisValue`)) _returnvalue) false false)
  (`/Engine/EditorBlueprintResources/StandardMacros.Gate` true :!label _label
    (:`Exit`
      (`self.K2_AddActorWorldOffset` (`self.Player 2`) (* (`KismetMathLibrary.MakeVector` (`self.GetInputAxisValue`) 0.0 (`self.GetInputAxisValue`)) _returnvalue) false false))))

(event `Key|SpaceBar`
  (params (Key :type "Key Structure"))
  ;[0.5 1 0.25] Cursor "Click"
  (:`Pressed`
    (`/Game/Player/Cursor_BP.Click` (`self.Player 1`))))

(event `Key|J`
  (params (Key :type "Key Structure"))
  ;[0.5 1 0.25] Cursor "Click"
  (:`Pressed`
    (`/Game/Player/Cursor_BP.Click` (`self.Player 2`))))

(fn `UserConstructionScript`)