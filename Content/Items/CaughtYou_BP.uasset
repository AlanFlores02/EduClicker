(event `self.ReceiveBeginPlay`
  (`KismetSystemLibrary.K2_SetTimerDelegate` (delegate `Fade Away`) 0.1 true))

(event `Fade Away`
  (bind _output_get (set `self.Alpha` (- (`self.Alpha`) 0.1)))
  (`PaperSpriteComponent.SetSpriteColor` (`self.RenderComponent`) (`KismetMathLibrary.MakeColor` 1.0 1.0 1.0 _output_get))
  (if (<= _output_get 0.0)
    (`self.K2_DestroyActor`)))

(fn `UserConstructionScript`)