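; Item_BP is a drifting Mario or Luigi sprite in a find-Luigi click game, wrapping around screen borders.
; Clicks arrive as AnyDamage: Luigi spawns CaughtYou_BP, damages the clicker, hides and notifies Background_BP, while Mario spawns WrongPerson_BP and plays regret audio.
; Reset restores Luigi as Mario and cycles the movement pattern through timer-driven zig-zags, faster straight motion and circular drift.
; ReturnToLuigi turns an item into the target.
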(event `self.ReceiveBeginPlay`
  (bind _returnvalue (`KismetSystemLibrary.K2_SetTimer` null "Zig-zag Movement" 2.0 true))
  (bind _output_get (set `self.Handle` _returnvalue))
  (`KismetSystemLibrary.K2_PauseTimerHandle` _output_get)
  ;[0 1 0] Set Initial Luigi
  (if (`self.Luigi`)
    (`self.Return To Luigi`)))

(event `self.ReceiveAnyDamage`
  (params (Damage :type "Float (single-precision)") (DamageType :type "DamageType Object Reference") (InstigatedBy :type "Controller Object Reference") (DamageCauser :type "Actor Object Reference"))
  (bind _returnvalue (`self.GetTransform`))
  ;[1 0.1 0.1] Event "Click"
  (if (`self.Luigi`)
    (`|SpawnActorFromClass` "/Game/Items/CaughtYou_BP.CaughtYou_BP_C" _returnvalue "AlwaysSpawn" "OverrideRootScale" null null)
    (`GameplayStatics.ApplyDamage` DamageCauser 1.0)
    (`self.Deactivate`)
    (else
      (`|SpawnActorFromClass` "/Game/Items/WrongPerson_BP.WrongPerson_BP_C" _returnvalue "AlwaysSpawn" "OverrideRootScale" null null)
      (`GameplayStatics.PlaySound2D` "/Game/Items/SFX/Mario_Regret.Mario_Regret" 1.0 1.0 0.0 null null))))

(event `self.ReceiveTick`
  (params (DeltaSeconds :type "Float (single-precision)"))
  (bind (_returnvalue_x _returnvalue_y _returnvalue_z) (`KismetMathLibrary.BreakVector` (`self.K2_GetActorLocation`)))
  (`|ExecutionSequence`
    (:`then_0`
      ;[1 1 0.5] Move in a straight line
      (`self.K2_AddActorWorldOffset` (* (`self.Basic Movement`) DeltaSeconds)))
    (:`then_1`
      ;[0.5 1 0.5] Special Movement
      (if (== 3 (`self.Pattern`))
        (`self.Circular Movement`)))
    (:`then_2`
      ;[0.2 0.2 1] Loop at screen borders
      (bind _new_pos (`self.Check Pos` 3400.0 _returnvalue_x)) ; Horizontal
      (bind _new_pos_2 (`self.Check Pos` 2000.0 _returnvalue_z)) ; Vertical
      (`self.K2_SetActorLocation` (`KismetMathLibrary.MakeVector` _new_pos 0.0 _new_pos_2)))))

(fn `Check Pos`
  (params (Limit :type "Float (double-precision)") (Pos :type "Float (double-precision)"))
  (returns (`New Pos` :type "Float (double-precision)"))
  (if (< Limit (`KismetMathLibrary.Abs` Pos))
    (return (* -0.95 Pos))
    (else
      (return Pos))))

(fn `Circular Movement`
  (locals (Speed :type "Float (double-precision)" :default 2000.0))
  (bind _returnvalue (`GameplayStatics.GetWorldDeltaSeconds`))
  (bind _speed (`local.Speed`))
  (bind _output_get (set `self.Time` (+ (`self.Time`) _returnvalue)))
  (`self.K2_AddActorWorldOffset` (* (`KismetMathLibrary.MakeVector` (* (`KismetMathLibrary.Cos` _output_get) _speed) 0.0 (* _speed (`KismetMathLibrary.Sin` _output_get))) _returnvalue)))

(fn `Deactivate`
  (`SceneComponent.SetVisibility` (`self.RenderComponent`) false false)
  (`self.SetActorEnableCollision` false)
  (bind _returnvalue (`GameplayStatics.GetActorOfClass` "/Game/Background/Background_BP.Background_BP_C"))
  (`/Game/Background/Background_BP.Luigi Found` _returnvalue))

(fn `Movement Three`)

(fn `Reset`
  (locals (`New Speed` :type "Float (double-precision)"))
  (bind _rendercomponent (`self.RenderComponent`))
  (bind _handle (`self.Handle`))
  (`|ExecutionSequence`
    (:`then_0`
      ;[0.2 0.4 0.2] Restore Deactivated Items
      (if (`self.Luigi`)
        (set `self.Luigi` false)
        (`SceneComponent.SetVisibility` _rendercomponent true false)
        (`self.SetActorEnableCollision` true)
        (`PaperSpriteComponent.SetSprite` _rendercomponent "/Game/Items/Sprites/Mario_Idle_Sprite.Mario_Idle_Sprite")))
    (:`then_1`
      ;[1 0.4 0.2] Change Movement Pattern
      (bind _result (`/Engine/EditorBlueprintResources/StandardMacros.IncrementInt` (`self.Pattern`))
        (:`  `
          (if (> _result 3)
            (set `self.Pattern` 0)))))
    (:`then_2`
      (switch `int` (`self.Pattern`)
        (:`0`
          (`KismetSystemLibrary.K2_UnPauseTimerHandle` _handle))
        (:`2`
          (`KismetSystemLibrary.K2_PauseTimerHandle` _handle)
          (set `local.New Speed` 2.0)
          (set `self.Basic Movement` (* (`self.Basic Movement`) (`local.New Speed`)) :!label _label))
        (:`3`
          (set `local.New Speed` 0.5)
          (goto _label))))))

(fn `Return To Luigi`
  (set `self.Luigi` true)
  (`PaperSpriteComponent.SetSprite` (`self.RenderComponent`) "/Game/Items/Sprites/Luigi_Idle_Sprite.Luigi_Idle_Sprite"))

(fn `UserConstructionScript`)

(fn `Zig-zag Movement`
  (locals (Mult :type "Vector Structure" :default (1.0 1.0 1.0)))
  (set `self.Basic Movement` (* (`self.Basic Movement`) (select `int` (`self.Pattern`) :`0` (-1.0 1.0 1.0) :`1` (1.0 1.0 -1.0) :!type "Vector Structure"))))